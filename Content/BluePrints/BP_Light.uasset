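; BP_Light is a light Blueprint that switches its spot light on and off according to a time value.
; Each Tick runs the parent Tick, then checks whether ParentTime falls within a fixed range.
; The SpotLight intensity is set to full brightness inside that window and to zero outside it, reapplied every frame with no fade.
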(event EventBeginPlay
  (|CallParentFunction) ; This node is disabled and will not be called.\nDrag off pins to build functionality.
)

(event Collision|EventActorBeginOverlap
  (params (OtherActor :type Actor%20Object%20Reference))
  (|CallParentFunction OtherActor) ; This node is disabled and will not be called.\nDrag off pins to build functionality.
)

(event EventTick
  (params (DeltaSeconds :type Float%20%28single-precision%29))
  (bind _spotlight (Variables|Default|GetSpotLight))
  (|CallParentFunction DeltaSeconds)
  (if (Math|Float|InRange(Float) (Variables|Default|GetParentTime) 12.0 2e+01)
    (Rendering|Components|Light|SetIntensity _spotlight 6e+03)
    (else
      (Rendering|Components|Light|SetIntensity _spotlight 0.0))))

(fn ConstructionScript
  (|CallParentFunction))