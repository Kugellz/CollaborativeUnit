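; Environment manager that runs a single day clock, rotating the light source and updating the sky as time passes.
; A fast looping timer advances Time, scaled by hour length, until DayLength stops it.
; Whenever Time lands near a multiple of 1000, it sets the Hour and notifies BPI_TimeListener actors gathered at BeginPlay.
; Time and hour values print on screen.
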(event Custom|AdvanceTime
  (if (Variables|Time|GetTimeProgress?)
    (Variables|Time|SetTime (+ (Variables|Time|GetTime) (/ 1e+01 (Variables|Time|GetHourLengthInSeconds))))
    (Development|PrintString (Utilities|String|ToString(Float) (Variables|Time|GetTime)) true true "(R=0.000000,G=0.660000,B=1.000000,A=1.000000)" 0.05)
    (Transformation|SetActorRotation (Variables|Object|GetLight%20Source) (Math|Rotator|MakeRotator 0.0 (* (Variables|Time|GetTime) -0.03) 0.0))
    (Default|UpdateSunDirection (Variables|Object|GetSkyLight))
    (if (Math|Float|NearlyEqual(Float) (/ (Variables|Time|GetTime) 1e+03) (Math|Conversions|ToFloat(Integer) (Math|Float|Round (/ (Variables|Time|GetTime) 1e+03))) 0.0001)
      (Development|PrintString (Utilities|String|ToString(Float) (Math|Conversions|ToFloat(Integer) (Math|Float|Round (/ (Variables|Time|GetTime) 1e+03)))) true true "(R=1.000000,G=0.000000,B=0.005718,A=1.000000)" 0.2)
      (Variables|Time|SetHour (Math|Float|Round (/ (Variables|Time|GetTime) 1e+03)))
      (CallFunction|UpdateTimeListeners))
    (if (>= (Variables|Time|GetTime) (Variables|Time|GetDayLength))
      (CallFunction|DayEnd))))

(event Custom|DayEnd
  (Variables|Time|SetTimeProgress? false))

(event Custom|DayStart
  (Variables|Time|SetTime 0.0)
  (Variables|Time|SetHour 0)
  (Variables|Time|SetTimeProgress? true))

(event EventBeginPlay
  (bind _outactors (Actor|GetAllActorswithInterface "/Game/BluePrints/Interfaces/BPI_TimeListener.BPI_TimeListener_C"))
  (Variables|Time|SetTimeListeners _outactors)
  (Utilities|Time|SetTimerbyEvent (delegate Custom|AdvanceTime) 0.01 true)
  (CallFunction|DayStart))

(fn ConstructionScript)

(fn UpdateTimeListeners
  (for _array_element (Variables|Time|GetTimeListeners)
    (Class|BPITimeListener|TimeUpdated(Message) _array_element (Variables|Time|GetHour))))