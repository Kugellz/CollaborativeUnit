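; BP_UniformSplineMesh is a spline actor that lays a static mesh along its path in repeated, evenly spaced sections.
; The construction script scales section length by the actor's scale on the forward axis, then derives the section count from spline length and spacing.
; Each spline mesh takes positions and length-clamped tangents from distances along the spline, offset by clamped random spacing and section variation, with query-only collision.
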(event EventBeginPlay)

(event Collision|EventActorBeginOverlap
  (params (OtherActor :type Actor%20Object%20Reference)))

(event EventTick
  (params (DeltaSeconds :type Float%20%28single-precision%29)))

(fn ConstructionScript
  (bind _returnvalue (Transformation|GetActorScale3D))
  (bind _spacingrandomisation (Variables|Default|GetSpacingRandomisation))
  (bind _spacing (Variables|Default|GetSpacing))
  (bind _sectionrandomisation (Variables|Default|GetSectionRandomisation))
  (bind _spline (Variables|Default|GetSpline))
  (bind _returnvalue_2 (Math|Float|Absolute(Float) _sectionrandomisation))
  (bind _returnvalue_3 (Math|Float|Absolute(Float) _spacingrandomisation))
  (bind _returnvalue_4 (* _spacing -1.0))
  (bind _returnvalue_5 (* _returnvalue_3 -1.0))
  (bind _returnvalue_6 (Math|Random|RandomFloatinRange _returnvalue_5 _returnvalue_3))
  (bind _returnvalue_7 (Math|Float|Clamp(Float) _returnvalue_6 _returnvalue_4 _spacing))
  (Variables|Default|SetSectionLength (* (Variables|Default|GetSectionLength) (Utilities|Select :Index (Variables|Default|GetForwardAxis) :X (.x _returnvalue) :Y (.y _returnvalue) :Z (.z _returnvalue))))
  (for _index (range 0 (Math|Float|Truncate (/ (Spline|GetSplineLength (Variables|Default|GetSpline)) (+ (Variables|Default|GetSectionLength) (Variables|Default|GetSpacing)))))
    (bind _returnvalue_8 (AddComponent|AddSplineMeshComponent false))
    (Components|StaticMesh|SetStaticMesh _returnvalue_8 (Variables|Default|GetMesh))
    (SplineMesh|SetForwardAxis _returnvalue_8 (Variables|Default|GetForwardAxis) true)
    (Transformation|AttachComponentToComponent _returnvalue_8 (Variables|Default|GetSpline) "None" "KeepRelative" "KeepRelative" "KeepRelative" true)
    (SplineMesh|SetStartandEnd _returnvalue_8 (Spline|GetLocationatDistanceAlongSpline _spline (+ (* _index (+ (Variables|Default|GetSectionLength) (Variables|Default|GetSpacing))) _returnvalue_7) "Local") (Math|Vector|ClampVectorSize (Spline|GetTangentatDistanceAlongSpline _spline (+ (* _index (+ (Variables|Default|GetSectionLength) (Variables|Default|GetSpacing))) _returnvalue_7) "Local") 0.0 (Variables|Default|GetSectionLength)) (Spline|GetLocationatDistanceAlongSpline _spline (+ (- (* (+ _index 1) (+ (Variables|Default|GetSectionLength) (Variables|Default|GetSpacing))) (Variables|Default|GetSpacing)) _returnvalue_7 (Math|Float|Clamp(Float) (Math|Random|RandomFloatinRange (* _returnvalue_2 -1.0) _returnvalue_2) (* (Variables|Default|GetSectionLength) -1.0) (Variables|Default|GetSectionLength))) "Local") (Math|Vector|ClampVectorSize (Spline|GetTangentatDistanceAlongSpline _spline (+ (- (* (+ _index 1) (+ (Variables|Default|GetSectionLength) (Variables|Default|GetSpacing))) (Variables|Default|GetSpacing)) _returnvalue_7 (Math|Float|Clamp(Float) (Math|Random|RandomFloatinRange (* _returnvalue_2 -1.0) _returnvalue_2) (* (Variables|Default|GetSectionLength) -1.0) (Variables|Default|GetSectionLength))) "Local") 0.0 (Variables|Default|GetSectionLength)) true :!class /Script/Engine.SplineMeshComponent)
    (Collision|SetCollisionEnabled _returnvalue_8 "QueryOnly")))