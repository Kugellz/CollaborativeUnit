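; Interactable object Blueprint that completes a task for the character interacting with it.
; Interact stores the character, prints its name as debug text, then after a short delay casts it to ThirdPersonCharacter and calls TaskComplete with its TaskData and itself.
; TimeUpdated stores the incoming time and compares it to TimeToRelease, but the branch does nothing.
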(event EventInteract
  (params (CharacterRef :type Third%20Person%20Character%20Object%20Reference))
  (bind _output_get (Variables|Default|SetHeld%20Character CharacterRef))
  (Development|PrintString (Utilities|String|Append "Interacted with: " (Utilities|GetDisplayName _output_get)) true true "(R=1.000000,G=0.000000,B=0.643363,A=1.000000)")
  (Utilities|FlowControl|Delay 1.0)
  (bind _asthird_person_character (Utilities|Casting|CastToThirdPersonCharacter _output_get))
  (Default|TaskComplete _asthird_person_character (Variables|Default|GetTaskData) self))

(event EventTimeUpdated
  (params (Time :type Integer) (Hour :type Integer) (Minute :type Integer))
  (bind _output_get (Variables|Default|SetTime Time))
  (if (>= _output_get (Variables|Default|GetTimeToRelease))
    _))

(fn ConstructionScript)